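; Component that makes its owning actor interactable, letting it be picked up, dropped or triggered.
; Pickup saves each primitive component's physics state, disables simulation, then snaps the actor to the interactor's holding socket with a relative offset.
; Drop detaches the actor in world space and restores the saved physics states by array index.
; Interact only fires the OnInteract dispatcher.
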(event EventBeginPlay
  ;[0.0502 1 0] BeginPlay
  (Variables|Default|SetInteractableObject (Components|GetOwner)))

(fn PickupInteractable
  (params (Interactor :type Scene%20Component%20Object%20Reference))
  (Utilities|Array|Clear (Variables|Default|GetbHoldedObjectSavedPhysics))
  (for _array_element (Actor|GetComponentsByClass (Variables|Default|GetInteractableObject) "/Script/Engine.PrimitiveComponent")
    (Utilities|Array|Add (Variables|Default|GetbHoldedObjectSavedPhysics) (Class|SceneComponent|IsAnySimulatingPhysics _array_element))
    (Physics|SetSimulatePhysics _array_element false))
  (Transformation|AttachComponentToComponent (Variables|Default|GetInteractableObject) Interactor (Variables|Settings|GetInteractorHoldingSocketName) "SnapToTarget" "SnapToTarget" "SnapToTarget" true)
  (Transformation|SetActorRelativeTransform (Variables|Default|GetInteractableObject) (Variables|Settings|GetHeldObjectOffset) false false))

(fn DropInteractable
  (bind _interactableobject (Variables|Default|GetInteractableObject))
  (Transformation|DetachFromActor _interactableobject "KeepWorld" "KeepWorld" "KeepWorld")
  (for (_array_element _array_index) (Actor|GetComponentsByClass _interactableobject "/Script/Engine.PrimitiveComponent")
    (Physics|SetSimulatePhysics _array_element (Utilities|Array|Get(acopy) (Variables|Default|GetbHoldedObjectSavedPhysics) _array_index))))

(fn Interact
  (Default|CallOnInteract))